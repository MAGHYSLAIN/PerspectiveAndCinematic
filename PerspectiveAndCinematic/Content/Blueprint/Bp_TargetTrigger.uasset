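; Bp_TargetTrigger is a trigger actor that detects an overlap with Box_Look while Box is overlapped, with no filter on the overlapping actor.
; Box sets and clears In00, which gates Box_Look's begin overlap to latch In01, a flag that is never reset.
; Tick prints a debug "Hello" while In01 is set.
; A SetViewTargetWithBlend camera switch is present but unconnected, and the Camera references are unused.
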(event `self.Box.OnComponentBeginOverlap`
  (params (OverlappedComponent :type "PrimitiveComponent Object Reference") (OtherActor :type "Actor Object Reference") (OtherComp :type "PrimitiveComponent Object Reference") (OtherBodyIndex :type Integer) (bFromSweep :type Boolean) (SweepResult :type "HitResult Structure (by ref)"))
  (set `self.In_00` true))

(event `self.Box.OnComponentEndOverlap`
  (params (OverlappedComponent :type "PrimitiveComponent Object Reference") (OtherActor :type "Actor Object Reference") (OtherComp :type "PrimitiveComponent Object Reference") (OtherBodyIndex :type Integer))
  (set `self.In_00` false))

(event `self.Box_Look.OnComponentBeginOverlap`
  (params (OverlappedComponent :type "PrimitiveComponent Object Reference") (OtherActor :type "Actor Object Reference") (OtherComp :type "PrimitiveComponent Object Reference") (OtherBodyIndex :type Integer) (bFromSweep :type Boolean) (SweepResult :type "HitResult Structure (by ref)"))
  (if (`self.In_00`)
    (set `self.In_01` true)))

(event `self.ReceiveTick`
  (params (DeltaSeconds :type "Float (single-precision)"))
  (if (`self.In_01`)
    (`KismetSystemLibrary.PrintString` "Hello")))

(fn `UserConstructionScript`)